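; AI kunai projectile Blueprint that damages Manne_BP characters on contact.
; Tick runs latent Delays that enable the capsule's query and physics collision shortly after spawn, then destroy the actor if it hits nothing within about ten seconds.
; A capsule overlap with a Manne_BP or subclass spawns a hit particle, briefly waits, applies random damage within a fixed range, and destroys the kunai.
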(event OnComponentBeginOverlap(CollisionCapsule)
  (params (OtherActor :type Actor%20Object%20Reference) (OtherComp :type Primitive%20Component%20Object%20Reference) (OtherBodyIndex :type Integer) (bFromSweep :type Boolean) (SweepResult :type Hit%20Result%20Structure%20%28by%20ref%29))
  ;[0.6059 0.6434 1] On Begin Overlap with TC
  (if (Utilities|ClassIsChildOf (Utilities|GetClass OtherActor) "/Game/TheArtOfCombat/CombatSystem/Blueprints/CharacterBlueprints/Manne/_Parent/Manne_BP.Manne_BP_C")
    (Effects|SpawnEmitteratLocation "/Game/TheArtOfCombat/CombatSystem/Particles/P_Kunai_Hit.P_Kunai_Hit" (Transformation|GetWorldLocation (Variables|Default|GetCollision%20Capsule)))
    (Utilities|FlowControl|Delay 0.05)
    (CallFunction|DealDamage)
    (Actor|DestroyActor)))

(event Custom|Deal%20Damage
  ;[0.8926 1 0.3959] Deal Damage
  (Game|Damage|ApplyDamage (stale OnComponentBeginOverlap(CollisionCapsule) OtherActor) (Math|Random|RandomFloatinRange 1e+01 2e+01) 0 0))

(event EventBeginPlay)

(event Collision|EventActorBeginOverlap
  (params (OtherActor :type Actor%20Object%20Reference)))

(event EventTick
  (params (DeltaSeconds :type Float%20%28single-precision%29))
  (Utilities|FlowControl|Delay 0.2)
  (Collision|SetCollisionEnabled (Variables|Default|GetCollision%20Capsule) "QueryAndPhysics")
  (Utilities|FlowControl|Delay 1e+01)
  (Actor|DestroyActor))

(fn ConstructionScript)