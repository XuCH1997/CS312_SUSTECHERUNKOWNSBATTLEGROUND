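; Battle-royale safe zone that shrinks in five stages and poisons the player character while outside the outer circle.
; A BeginPlay delay chain halves and randomly moves the In circle, timelines lerp Out onto it, and poison damage doubles each stage.
; Out overlaps gate roughly once-per-second damage in Tick.
; The last shrink prints a win message and exits; the game-over UI branch is hard-coded false and HUD/health initialization is disconnected.
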(event OnComponentBeginOverlap(Out)
  (params (OverlappedComponent :type Primitive%20Component%20Object%20Reference) (OtherActor :type Actor%20Object%20Reference) (OtherComp :type Primitive%20Component%20Object%20Reference) (OtherBodyIndex :type Integer) (bFromSweep :type Boolean) (SweepResult :type Hit%20Result%20Structure%20%28by%20ref%29))
  ;[1 1 1] 进入外圈关闭伤害
  (if (== OtherActor (Game|GetPlayerCharacter 0))
    (Variables|Default|SetHaveHealth true)))

(event OnComponentEndOverlap(Out)
  (params (OverlappedComponent :type Primitive%20Component%20Object%20Reference) (OtherActor :type Actor%20Object%20Reference) (OtherComp :type Primitive%20Component%20Object%20Reference) (OtherBodyIndex :type Integer))
  ;[1 1 1] 进入外圈关闭伤害
  (if (== OtherActor (Game|GetPlayerCharacter 0))
    (Variables|Default|SetHaveHealth false)))

(event EventTick
  (params (DeltaSeconds :type Float%20%28single-precision%29))
  (Utilities|FlowControl|Sequence
    (:then_0
      (if false
        ;[1 1 1] 显示结束UI
        (Utilities|FlowControl|DoOnce false
          (:Completed
            (Widget|RemovefromParent (Variables|Default|GetPlayerHUD_Ref))
            (bind _returnvalue (UserInterface|CreateWidget "/Game/UMG/Tips.Tips_C"))
            (UserInterface|Viewport|AddtoViewport _returnvalue 0)
            (Variables|/Script/Engine.PlayerController|SetbShowMouseCursor (Game|GetPlayerController 0) true)))
        (else
          ;[1 1 1] 角色减血
          (if (not (Variables|Default|GetHaveHealth))
            (Utilities|FlowControl|DoOnce false :!label _label
              (:Completed
                (Utilities|FlowControl|Sequence
                  (:then_0
                    (Utilities|FlowControl|Delay 1.0)
                    (goto _label Reset))
                  (:then_1
                    (bind _output_get (Variables|Default|SetCharacterHealth (- (Variables|Default|GetCharacterHealth) (Variables|Default|GetPoisonDamage))))
                    (Development|PrintString (Utilities|String|ToString(Float) _output_get) true false)))))))))
    (:then_1
      ;[1 1 1] 角色当前状态
      (if (<= (Variables|Default|GetCharacterHealth) 0.0)
        (Variables|Default|SetIsStop true)
        (else
          (Variables|Default|SetIsStop false))))))

(event EventBeginPlay
  (bind _in (Variables|Default|GetIn))
  (bind _out (Variables|Default|GetOut))
  (bind _in_2 (Variables|Default|GetIn))
  (bind _out_2 (Variables|Default|GetOut))
  (bind _out_3 (Variables|Default|GetOut))
  (bind _out_4 (Variables|Default|GetOut))
  (bind _in_3 (Variables|Default|GetIn))
  (bind _in_4 (Variables|Default|GetIn))
  (bind _out_5 (Variables|Default|GetOut))
  (bind _in_5 (Variables|Default|GetIn))
  (bind _out_6 (Variables|Default|GetOut))
  (bind _out_7 (Variables|Default|GetOut))
  (bind _out_8 (Variables|Default|GetOut))
  (bind _in_6 (Variables|Default|GetIn))
  (bind _in_7 (Variables|Default|GetIn))
  (bind _out_9 (Variables|Default|GetOut))
  (bind _in_8 (Variables|Default|GetIn))
  (bind _out_10 (Variables|Default|GetOut))
  (bind _out_11 (Variables|Default|GetOut))
  (bind _out_12 (Variables|Default|GetOut))
  (bind _in_9 (Variables|Default|GetIn))
  (bind _in_10 (Variables|Default|GetIn))
  (bind _out_13 (Variables|Default|GetOut))
  (bind _in_11 (Variables|Default|GetIn))
  (bind _out_14 (Variables|Default|GetOut))
  (bind _out_15 (Variables|Default|GetOut))
  (bind _out_16 (Variables|Default|GetOut))
  (bind _in_12 (Variables|Default|GetIn))
  (bind _in_13 (Variables|Default|GetIn))
  (bind _out_17 (Variables|Default|GetOut))
  (bind _in_14 (Variables|Default|GetIn))
  (bind _out_18 (Variables|Default|GetOut))
  (bind _out_19 (Variables|Default|GetOut))
  (bind _in_15 (Variables|Default|GetIn))
  (bind _returnvalue (Transformation|GetWorldLocation _in_10))
  (bind _returnvalue_2 (Transformation|GetWorldLocation _in_7))
  (bind _returnvalue_3 (Transformation|GetWorldLocation _in_13))
  (bind _returnvalue_4 (Transformation|GetWorldLocation _in))
  (bind _returnvalue_5 (Transformation|GetWorldLocation _in_4))
  (bind _relativescale3d (Variables|/Script/Engine.SceneComponent|GetRelativeScale3D _out_4))
  (bind _relativescale3d_2 (Variables|/Script/Engine.SceneComponent|GetRelativeScale3D _in_3))
  (bind _relativescale3d_3 (Variables|/Script/Engine.SceneComponent|GetRelativeScale3D _out_8))
  (bind _relativescale3d_4 (Variables|/Script/Engine.SceneComponent|GetRelativeScale3D _in_6))
  (bind _relativescale3d_5 (Variables|/Script/Engine.SceneComponent|GetRelativeScale3D _out_12))
  (bind _relativescale3d_6 (Variables|/Script/Engine.SceneComponent|GetRelativeScale3D _in_9))
  (bind _relativescale3d_7 (Variables|/Script/Engine.SceneComponent|GetRelativeScale3D _out_16))
  (bind _relativescale3d_8 (Variables|/Script/Engine.SceneComponent|GetRelativeScale3D _in_12))
  (bind _relativescale3d_9 (Variables|/Script/Engine.SceneComponent|GetRelativeScale3D _out_19))
  (bind _relativescale3d_10 (Variables|/Script/Engine.SceneComponent|GetRelativeScale3D _in_15))
  (bind (_x _y) (Math|Vector|BreakVector _returnvalue))
  (bind _returnvalue_6 (* _relativescale3d_7 25.0))
  (bind (_x_2 _y_2 _z) (Math|Vector|BreakVector _relativescale3d_8))
  (bind (_x_3 _y_3) (Math|Vector|BreakVector _returnvalue_2))
  (bind _returnvalue_7 (* _relativescale3d_5 25.0))
  (bind (_x_4 _y_4 _z_2) (Math|Vector|BreakVector _relativescale3d_6))
  (bind (_x_5 _y_5) (Math|Vector|BreakVector _returnvalue_3))
  (bind _returnvalue_8 (* _relativescale3d_9 25.0))
  (bind (_x_6 _y_6 _z_3) (Math|Vector|BreakVector _relativescale3d_10))
  (bind (_x_7 _y_7) (Math|Vector|BreakVector _returnvalue_4))
  (bind _returnvalue_9 (* _relativescale3d 25.0))
  (bind (_x_8 _y_8 _z_4) (Math|Vector|BreakVector _relativescale3d_2))
  (bind (_x_9 _y_9) (Math|Vector|BreakVector _returnvalue_5))
  (bind _returnvalue_10 (* _relativescale3d_3 25.0))
  (bind (_x_10 _y_10 _z_5) (Math|Vector|BreakVector _relativescale3d_4))
  (bind _x_11 (Math|Vector|BreakVector _returnvalue_7))
  (bind _x_12 (Math|Vector|BreakVector _returnvalue_6))
  (bind _x_13 (Math|Vector|BreakVector _returnvalue_8))
  (bind _x_14 (Math|Vector|BreakVector _returnvalue_9))
  (bind _x_15 (Math|Vector|BreakVector _returnvalue_10))
  (bind _returnvalue_11 (- 0.0 _x_11))
  (bind _returnvalue_12 (- 0.0 _x_12))
  (bind _returnvalue_13 (- 0.0 _x_13))
  (bind _returnvalue_14 (- 0.0 _x_14))
  (bind _returnvalue_15 (- 0.0 _x_15))
  (bind _returnvalue_16 (* _x_11 _x_11))
  (bind _returnvalue_17 (* _x_12 _x_12))
  (bind _returnvalue_18 (* _x_13 _x_13))
  (bind _returnvalue_19 (* _x_14 _x_14))
  (bind _returnvalue_20 (* _x_15 _x_15))
  (bind _returnvalue_21 (Math|Random|RandomFloatinRange _returnvalue_11 _x_11))
  (bind _returnvalue_22 (Math|Random|RandomFloatinRange _returnvalue_12 _x_12))
  (bind _returnvalue_23 (Math|Random|RandomFloatinRange _returnvalue_13 _x_13))
  (bind _returnvalue_24 (Math|Random|RandomFloatinRange _returnvalue_14 _x_14))
  (bind _returnvalue_25 (Math|Random|RandomFloatinRange _returnvalue_15 _x_15))
  (bind _returnvalue_26 (* _returnvalue_21 _returnvalue_21))
  (bind _returnvalue_27 (* _returnvalue_22 _returnvalue_22))
  (bind _returnvalue_28 (* _returnvalue_23 _returnvalue_23))
  (bind _returnvalue_29 (* _returnvalue_24 _returnvalue_24))
  (bind _returnvalue_30 (* _returnvalue_25 _returnvalue_25))
  (bind _returnvalue_31 (- _returnvalue_16 _returnvalue_26))
  (bind _returnvalue_32 (- _returnvalue_17 _returnvalue_27))
  (bind _returnvalue_33 (- _returnvalue_18 _returnvalue_28))
  (bind _returnvalue_34 (- _returnvalue_19 _returnvalue_29))
  (bind _returnvalue_35 (- _returnvalue_20 _returnvalue_30))
  (bind _returnvalue_36 (Math|Float|Sqrt _returnvalue_31))
  (bind _returnvalue_37 (Math|Float|Sqrt _returnvalue_32))
  (bind _returnvalue_38 (Math|Float|Sqrt _returnvalue_33))
  (bind _returnvalue_39 (Math|Float|Sqrt _returnvalue_34))
  (bind _returnvalue_40 (Math|Float|Sqrt _returnvalue_35))
  (Utilities|FlowControl|Delay 2.0)
  ;[1 1 1] 设置内圈位置大小
  (Development|PrintString "10s后开始缩圈" true true "(R=0.000000,G=0.000000,B=0.000000,A=1.000000)" 5.0)
  (Transformation|SetWorldScale3D _in_12 (Math|Vector|MakeVector (/ _x_2 2.0) (/ _y_2 2.0) _z))
  (Transformation|SetWorldLocation (Variables|Default|GetIn) (Math|Vector|MakeVector (+ _returnvalue_22 _x) (+ _y (Math|Random|RandomFloatinRange (- 0.0 _returnvalue_37) _returnvalue_37)) 0.0) false false)
  (Utilities|FlowControl|Delay 4e+01)
  ;[1 1 1] 外圈跟随收缩
  (Utilities|FlowControl|Sequence
    (:then_0
      (Utilities|FlowControl|Delay 2e+01)
      (Variables|Default|SetPoisonDamage (* (Variables|Default|GetPoisonDamage) 2.0))
      ;[1 1 1] 设置内圈位置大小
      (Transformation|SetWorldScale3D _in_3 (Math|Vector|MakeVector (/ _x_8 2.0) (/ _y_8 2.0) _z_4))
      (Transformation|SetWorldLocation (Variables|Default|GetIn) (Math|Vector|MakeVector (+ _returnvalue_24 _x_7) (+ _y_7 (Math|Random|RandomFloatinRange (- 0.0 _returnvalue_39) _returnvalue_39)) 0.0) false false)
      (Utilities|FlowControl|Delay 4e+01)
      ;[1 1 1] 外圈跟随收缩
      (Utilities|FlowControl|Sequence
        (:then_0
          (Utilities|FlowControl|Delay 2e+01)
          (Variables|Default|SetPoisonDamage (* (Variables|Default|GetPoisonDamage) 2.0))
          ;[1 1 1] 设置内圈位置大小
          (Transformation|SetWorldScale3D _in_9 (Math|Vector|MakeVector (/ _x_4 2.0) (/ _y_4 2.0) _z_2))
          (Transformation|SetWorldLocation (Variables|Default|GetIn) (Math|Vector|MakeVector (+ _returnvalue_21 _x_3) (+ _y_3 (Math|Random|RandomFloatinRange (- 0.0 _returnvalue_36) _returnvalue_36)) 0.0) false false)
          (Utilities|FlowControl|Delay 3e+01)
          ;[1 1 1] 外圈跟随收缩
          (Utilities|FlowControl|Sequence
            (:then_0
              (Utilities|FlowControl|Delay 2e+01)
              (Variables|Default|SetPoisonDamage (* (Variables|Default|GetPoisonDamage) 2.0))
              ;[1 1 1] 设置内圈位置大小
              (Transformation|SetWorldScale3D _in_6 (Math|Vector|MakeVector (/ _x_10 2.0) (/ _y_10 2.0) _z_5))
              (Transformation|SetWorldLocation (Variables|Default|GetIn) (Math|Vector|MakeVector (+ _returnvalue_25 _x_9) (+ _y_9 (Math|Random|RandomFloatinRange (- 0.0 _returnvalue_40) _returnvalue_40)) 0.0) false false)
              (Utilities|FlowControl|Delay 3e+01)
              ;[1 1 1] 外圈跟随收缩
              (Utilities|FlowControl|Sequence
                (:then_0
                  (Utilities|FlowControl|Delay 2e+01)
                  (Variables|Default|SetPoisonDamage (* (Variables|Default|GetPoisonDamage) 2.0))
                  ;[1 1 1] 设置内圈位置大小
                  (Transformation|SetWorldScale3D _in_15 (Math|Vector|MakeVector (/ _x_6 2.0) (/ _y_6 2.0) _z_3))
                  (Transformation|SetWorldLocation (Variables|Default|GetIn) (Math|Vector|MakeVector (+ _returnvalue_23 _x_5) (+ _y_5 (Math|Random|RandomFloatinRange (- 0.0 _returnvalue_38) _returnvalue_38)) 0.0) false false)
                  (Utilities|FlowControl|Delay 3e+01)
                  ;[1 1 1] 外圈跟随收缩
                  (Utilities|FlowControl|Sequence
                    (:then_0
                      (Utilities|FlowControl|Delay 2e+01)
                      (Variables|Default|SetPoisonDamage (* (Variables|Default|GetPoisonDamage) 2.0)))
                    (:then_1
                      (bind _output_get (Variables|Default|SetOutLocation (Transformation|GetWorldLocation _out_18)))
                      (bind _output_get_2 (Variables|Default|SetOutScale (Transformation|GetWorldScale _out_18)))
                      (bind _time (Timeline|时间轴_2 Play)
                        (:Update
                          (Transformation|SetWorldScale3D _out_17 (Math|Vector|Lerp(Vector) _output_get_2 (Transformation|GetWorldScale _in_14) _time))
                          (Transformation|SetWorldLocation _out_17 (Math|Vector|Lerp(Vector) _output_get (Transformation|GetWorldLocation _in_14) _time) false false))
                        (:Finished
                          (Development|PrintText "牛逼，你赢了" true false "(R=1.000000,G=1.000000,B=1.000000,A=1.000000)")
                          (Utilities|FlowControl|Delay 3.0)
                          (Development|ExecuteConsoleCommand "exit"))))))
                (:then_1
                  (bind _output_get_3 (Variables|Default|SetOutLocation (Transformation|GetWorldLocation _out_6)))
                  (bind _output_get_4 (Variables|Default|SetOutScale (Transformation|GetWorldScale _out_6)))
                  (bind _time_2 (Timeline|时间轴_3 Play)
                    (:Update
                      (Transformation|SetWorldScale3D _out_5 (Math|Vector|Lerp(Vector) _output_get_4 (Transformation|GetWorldScale _in_5) _time_2))
                      (Transformation|SetWorldLocation _out_5 (Math|Vector|Lerp(Vector) _output_get_3 (Transformation|GetWorldLocation _in_5) _time_2) false false))
                    (:Finished
                      (Development|PrintText "5s后刷圈" true false "(R=1.000000,G=1.000000,B=1.000000,A=1.000000)")
                      (Variables|Default|SetOutLocation (Transformation|GetWorldLocation _out_7))
                      (Variables|Default|SetOutScale (Transformation|GetWorldScale _out_7)))))))
            (:then_1
              (bind _output_get_5 (Variables|Default|SetOutLocation (Transformation|GetWorldLocation _out_10)))
              (bind _output_get_6 (Variables|Default|SetOutScale (Transformation|GetWorldScale _out_10)))
              (bind _time_3 (Timeline|时间轴_1 Play)
                (:Update
                  (Transformation|SetWorldScale3D _out_9 (Math|Vector|Lerp(Vector) _output_get_6 (Transformation|GetWorldScale _in_8) _time_3))
                  (Transformation|SetWorldLocation _out_9 (Math|Vector|Lerp(Vector) _output_get_5 (Transformation|GetWorldLocation _in_8) _time_3) false false))
                (:Finished
                  (Development|PrintText "5s后刷圈" true false "(R=1.000000,G=1.000000,B=1.000000,A=1.000000)")
                  (Variables|Default|SetOutLocation (Transformation|GetWorldLocation _out_11))
                  (Variables|Default|SetOutScale (Transformation|GetWorldScale _out_11)))))))
        (:then_1
          (bind _output_get_7 (Variables|Default|SetOutLocation (Transformation|GetWorldLocation _out_2)))
          (bind _output_get_8 (Variables|Default|SetOutScale (Transformation|GetWorldScale _out_2)))
          (bind _time_4 (Timeline|时间轴_0 Play)
            (:Update
              (Transformation|SetWorldScale3D _out (Math|Vector|Lerp(Vector) _output_get_8 (Transformation|GetWorldScale _in_2) _time_4))
              (Transformation|SetWorldLocation _out (Math|Vector|Lerp(Vector) _output_get_7 (Transformation|GetWorldLocation _in_2) _time_4) false false))
            (:Finished
              (Development|PrintText "5s后刷圈" true false "(R=1.000000,G=1.000000,B=1.000000,A=1.000000)")
              (Variables|Default|SetOutLocation (Transformation|GetWorldLocation _out_3))
              (Variables|Default|SetOutScale (Transformation|GetWorldScale _out_3)))))))
    (:then_1
      (bind _output_get_9 (Variables|Default|SetOutLocation (Transformation|GetWorldLocation _out_14)))
      (bind _output_get_10 (Variables|Default|SetOutScale (Transformation|GetWorldScale _out_14)))
      (bind _time_5 (Timeline|Refresh Play)
        (:Update
          (Transformation|SetWorldScale3D _out_13 (Math|Vector|Lerp(Vector) _output_get_10 (Transformation|GetWorldScale _in_11) _time_5))
          (Transformation|SetWorldLocation _out_13 (Math|Vector|Lerp(Vector) _output_get_9 (Transformation|GetWorldLocation _in_11) _time_5) false false))
        (:Finished
          (Development|PrintText "5s后刷圈" true false "(R=1.000000,G=1.000000,B=1.000000,A=1.000000)")
          (Variables|Default|SetOutLocation (Transformation|GetWorldLocation _out_15))
          (Variables|Default|SetOutScale (Transformation|GetWorldScale _out_15)))))))

(fn ConstructionScript
  (bind _outsize (Variables|Default|GetOutSize))
  (bind _insize (Variables|Default|GetInSize))
  (Transformation|SetWorldScale3D (Variables|Default|GetIn) (Math|Vector|MakeVector _insize _insize (/ _insize 0.001)))
  (Transformation|SetWorldScale3D (Variables|Default|GetOut) (Math|Vector|MakeVector _outsize _outsize (/ _outsize 0.001))))